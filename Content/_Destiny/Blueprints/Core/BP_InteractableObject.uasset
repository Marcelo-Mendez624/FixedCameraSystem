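; BP_InteractableObject is an interactable actor that is brought up to the player character for a focused view.
; StartFocus moves and attaches it to the character's ObjectAttachPoint, switches the view target to that character and ignores move and look input.
; StopFocus detaches it, restores its location from ObjectInitialPosition, blends back to the character's CurrentCameraActor and re-enables input.
; An OnEventTrigger binding made at BeginPlay only prints the event type.
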(event `InteractInterface.StartFocus`
  (params (Caller :type "Character Object Reference"))
  (bind _returnvalue (`GameplayStatics.GetPlayerController` 0))
  (bind _asbp_destiny_character (cast `/Game/_Destiny/Blueprints/Core/Character/BP_DestinyCharacter` Caller))
  (bind _objectattachpoint (`DestinyCharacter.ObjectAttachPoint` _asbp_destiny_character))
  (`self.K2_SetActorLocation` (`SceneComponent.K2_GetComponentLocation` _objectattachpoint))
  (`self.K2_AttachToComponent` _objectattachpoint "None" "KeepWorld" "KeepWorld" "KeepRelative")
  (`PlayerController.SetViewTargetWithBlend` _returnvalue _asbp_destiny_character 0.0 "VTBlend_Linear" 0.0 false)
  (`Controller.SetIgnoreMoveInput` _returnvalue true)
  (`Controller.SetIgnoreLookInput` _returnvalue true))

(event `InteractInterface.StopFocus`
  (params (Caller :type "Character Object Reference"))
  (bind _returnvalue (`GameplayStatics.GetPlayerController` 0))
  (`self.K2_DetachFromActor` self "KeepWorld" "KeepWorld" "KeepWorld")
  (`self.K2_SetActorLocation` (`self.ObjectInitialPosition`))
  (bind _asbp_destiny_character (cast `/Game/_Destiny/Blueprints/Core/Character/BP_DestinyCharacter` Caller))
  (`PlayerController.SetViewTargetWithBlend` _returnvalue (`DestinyCharacter.CurrentCameraActor` _asbp_destiny_character) 0.0 "VTBlend_Linear" 0.0 false)
  (`Controller.SetIgnoreMoveInput` _returnvalue false)
  (`Controller.SetIgnoreLookInput` _returnvalue false))

(event `self.ReceiveBeginPlay`
  (add `self.OnEventTrigger` (delegate `OnEventTrigger_Event`)))

(event `OnEventTrigger_Event` :!signature `self.OnEventTrigger`
  (params (EventType :type "EEventType Enum" :default "ETotemFound"))
  (`KismetSystemLibrary.PrintString` (`|GetEnumeratorNameAsString` EventType)))

(fn `UserConstructionScript`)